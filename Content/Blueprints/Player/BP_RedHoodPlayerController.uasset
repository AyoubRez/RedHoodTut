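; Player controller for the RedHood character in a side-scrolling movement setup along the world X axis.
; On BeginPlay it caches the possessed BP_Character_Base, adds the Enhanced Input mapping context, and creates the overlay widget, storing it on the character.
; Move and jump inputs are ignored while the character is attacking, and attack input is forwarded as AttackMessage.
; Movement input is rounded, and control yaw flips between facing directions based on acceleration sign.
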(event `self.ReceiveBeginPlay`
  (bind _asbp_character_base (cast `/Game/Blueprints/Characters/BP_Character_Base` (`self.K2_GetPawn`)))
  (set `self.ControlledCharacter` _asbp_character_base)
  (`EnhancedInputSubsystemInterface.AddMappingContext` (subsystem `EnhancedInputLocalPlayerSubsystem`) "/Game/Input/IMC_RedHood_Default.IMC_RedHood_Default" 0 (struct))
  (bind _returnvalue (`|CreateWidget` "/Game/Blueprints/UI/WBP_Overlay.WBP_Overlay_C" self))
  (bind _output_get (set `/Game/Blueprints/Characters/BP_Character_Base.Overlay` _returnvalue (`self.ControlledCharacter`)))
  (`UserWidget.AddToViewport` _output_get 0))

(event `EnhancedInput|/Game/Input/InputActions/IA_Move`
  (params (ActionValue :type "Float (double-precision)") (ElapsedSeconds :type "Float (double-precision)") (TriggeredSeconds :type "Float (double-precision)") (InputAction :type "InputAction Object Reference" :default "/Game/Input/InputActions/IA_Move.IA_Move"))
  (:`Triggered`
    (if (not (`/Game/Blueprints/Characters/BP_Character_Base.bIsAttacking` (`self.ControlledCharacter`)))
      (`self.Move`))))

(event `EnhancedInput|/Game/Input/InputActions/IA_Jump`
  (params (ActionValue :type Boolean) (ElapsedSeconds :type "Float (double-precision)") (TriggeredSeconds :type "Float (double-precision)") (InputAction :type "InputAction Object Reference" :default "/Game/Input/InputActions/IA_Jump.IA_Jump"))
  (:`Triggered`
    (if (not (`/Game/Blueprints/Characters/BP_Character_Base.bIsAttacking` (`self.ControlledCharacter`)))
      (`self.Character Jump` ActionValue))))

(event `EnhancedInput|/Game/Input/InputActions/IA_Attack`
  (params (ActionValue :type Boolean) (ElapsedSeconds :type "Float (double-precision)") (TriggeredSeconds :type "Float (double-precision)") (InputAction :type "InputAction Object Reference" :default "/Game/Input/InputActions/IA_Attack.IA_Attack"))
  (:`Triggered`
    (bind _controlledcharacter (`self.ControlledCharacter`)
      (:`then`
        (message `/Game/Blueprints/Interfaces/BPI_Player.Attack` _controlledcharacter))
      (:`else`))))

(fn `Character Jump`
  (params (InputActionValue :type Boolean))
  (bind _controlledcharacter (`self.ControlledCharacter`)
    (:`then`
      (if InputActionValue
        (`Character.Jump` _controlledcharacter)
        (else
          (`Character.StopJumping` _controlledcharacter))))
    (:`else`)))

(fn `Move`
  (`self.RotateController`)
  (`Pawn.AddMovementInput` (`self.ControlledCharacter`) (1.0 0.0 0.0) (`KismetMathLibrary.Conv_IntToDouble` (`KismetMathLibrary.Round` (`|GetInputActionValue`))) false))

(fn `RotateController`
  (bind _returnvalue_x (`KismetMathLibrary.BreakVector` (`CharacterMovementComponent.GetCurrentAcceleration` (`Character.CharacterMovement` (`self.ControlledCharacter`)))))
  (`/Engine/EditorBlueprintResources/StandardMacros.CompareFloat` _returnvalue_x
    (:`>`
      (`self.SetControlRotation` (`KismetMathLibrary.MakeRotator` 0.0)))
    (:`<`
      (`self.SetControlRotation` (`KismetMathLibrary.MakeRotator` 0.0 0.0 180.0)))))

(fn `UserConstructionScript`)