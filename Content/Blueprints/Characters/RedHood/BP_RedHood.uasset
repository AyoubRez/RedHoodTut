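; BP_RedHood is the Red Hood player character, handling a melee-style attack combo and health bar updates.
; Attack starts the combo, or queues the next hit if pressed during the window set by SetAttackWindow.
; ResetAttacking advances a queued combo or ends it, with the AttackCombo map supplying each step's override animation and damage.
; TakeDamage extends the parent's version to refresh the overlay's health bar.
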(event `/Game/Blueprints/Interfaces/BPI_Player.Attack`
  (bind _value (`BlueprintMapLibrary.Map_Find` (`self.AttackCombo`) (`self.AttackCount`)))
  (if (`self.bIsAttackWindowOpen`)
    (set `self.ComboActivated` true)
    (elif (not (`self.bIsAttacking`))
      (set `self.bIsAttacking` true)
      (`PaperZDAnimInstance.K2_PlayAnimationOverride` (`PaperZDAnimationComponent.AnimInstance` (`self.AnimationComponent`)) (break `/Game/Blueprints/Characters/RedHood/ST_AttackDamage` _value) "DefaultSlot" 1.0 0.0)
      (set `self.Damage` (`.Damage_5_A6EE1E8E45BB1AEF024CC1826D8F1FEE` (break `/Game/Blueprints/Characters/RedHood/ST_AttackDamage` _value))))))

(event `/Game/Blueprints/Interfaces/BPI_Player.ResetAttacking`
  (bind _value (`BlueprintMapLibrary.Map_Find` (`self.AttackCombo`) (`self.AttackCount`)))
  (if (`self.ComboActivated`)
    (bind _result (`/Engine/EditorBlueprintResources/StandardMacros.IncrementInt` (`self.AttackCount`))
      (:`  `
        (if (> _result (- (`BlueprintMapLibrary.Map_Length` (`self.AttackCombo`)) 1))
          (set `self.bIsAttacking` false)
          (set `self.AttackCount` 0)
          (set `self.ComboActivated` false))
        (`PaperZDAnimInstance.K2_PlayAnimationOverride` (`PaperZDAnimationComponent.AnimInstance` (`self.AnimationComponent`)) (break `/Game/Blueprints/Characters/RedHood/ST_AttackDamage` _value) "DefaultSlot" 1.0 0.0)
        (set `self.Damage` (`.Damage_5_A6EE1E8E45BB1AEF024CC1826D8F1FEE` (break `/Game/Blueprints/Characters/RedHood/ST_AttackDamage` _value)))
        (set `self.ComboActivated` false)))
    (else
      (set `self.bIsAttacking` false)
      (set `self.AttackCount` 0))))

(event `/Game/Blueprints/Interfaces/BPI_Player.SetAttackWindow`
  (params (bOpen :type Boolean))
  (set `self.bIsAttackWindowOpen` bOpen))

(fn `TakeDamage`
  (params (InDamage :type "Float (single-precision)"))
  (`parent.TakeDamage` InDamage)
  (bind _overlay (`self.Overlay`)
    (:`then`
      (`/Game/Blueprints/UI/WBP_PlayerHealthbar.SetHealthAttributeValues` (`/Game/Blueprints/UI/WBP_Overlay.PlayerHealthBar` _overlay) (`self.CurrentHealth`) (`self.MaxHealth`)))
    (:`else`)))

(fn `UserConstructionScript`)