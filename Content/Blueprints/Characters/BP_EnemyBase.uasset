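; BP_EnemyBase is a base enemy character Blueprint that links combat events to AI and animation.
; SetCombatTarget writes the target to the controller's Blackboard, and Attack triggers the attack animation.
; ChangeDirections turns the actor around with a 180-degree rotation, while Tick only calls its parent.
; Unconnected debug sphere draws for concentric ranges around the actor remain in the graph and never run.
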(event `self.ReceiveTick`
  (params (DeltaSeconds :type "Float (single-precision)"))
  (`parent.ReceiveTick` 0.0))

(event `/Game/Blueprints/Interfaces/BPI_Enemy.SetCombatTarget`
  (params (CombatTarget :type "Actor Object Reference"))
  (`BlackboardComponent.SetValueAsObject` (`AIBlueprintHelperLibrary.GetBlackboard` (`self.GetController`)) (`self.BB_Key_Combat_Target`) CombatTarget))

(event `/Game/Blueprints/Interfaces/BPI_Enemy.Attack`
  (`self.PlayAttackAnim`))

(fn `ChangeDirections`
  (`self.K2_SetActorRotation` (`KismetMathLibrary.ComposeRotators` (`self.K2_GetActorRotation`) (struct :`Yaw` 180.0))))

(fn `UserConstructionScript`)