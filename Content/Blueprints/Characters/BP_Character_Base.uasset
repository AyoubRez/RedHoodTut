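; Base character Blueprint providing shared melee attack, hit reaction and health logic.
; AttackBoxTrace box-traces between two marker components and calls GetHit on the character it strikes.
; GetHit subtracts clamped health, plays an override hit-react sequence, spawns particles and creates a floating damage-number widget projected above the character.
; Damage numbers require the hit character's own controller to be a PlayerController, cached at BeginPlay.
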(event `self.ReceiveBeginPlay`
  (set `self.PlayerController` (cast `PlayerController` (`self.GetController`) :!pure true)))

(event `self.ReceiveTick`
  (params (DeltaSeconds :type "Float (single-precision)")))

(fn `AttackBoxTrace`
  (bind _outhit (`KismetSystemLibrary.BoxTraceSingleForObjects` (`SceneComponent.K2_GetComponentLocation` (`self.BoxTraceStart`)) (`SceneComponent.K2_GetComponentLocation` (`self.BoxTraceEnd`)) (`self.TraceExtend`) (`self.BoxRotation`) (`self.TraceObjectTypes`)))
  (bind _asbp_character_base (cast `/Game/Blueprints/Characters/BP_Character_Base` (`.HitActor` (`GameplayStatics.BreakHitResult` _outhit))))
  (`self.GetHit` _asbp_character_base (`self.Damage`)))

(fn `CreateDamageNumber`
  (params (InDamage :type "Float (double-precision)") (Location :type "Vector Structure"))
  (locals (DamageNumber :type "/Game/Blueprints/UI/WBP_DamageNumber Object Reference"))
  (bind (_location_x _location_y _location_z) (`KismetMathLibrary.BreakVector` (`local.Location`)))
  (bind _damagenumber (`local.DamageNumber`))
  (bind _playercontroller (`self.PlayerController`)
    (:`then`
      (bind _returnvalue (`|CreateWidget` "/Game/Blueprints/UI/WBP_DamageNumber.WBP_DamageNumber_C" _playercontroller))
      (set `local.DamageNumber` _returnvalue)
      (`|ExecutionSequence`
        (:`then_0`
          (`/Game/Blueprints/UI/WBP_DamageNumber.SetDamageNumber` (`local.DamageNumber`) (`local.InDamage`) (`self.DamageNumberColorAndOpacity`)))
        (:`then_1`
          (`UserWidget.SetPositionInViewport` (`local.DamageNumber`) (`GameplayStatics.ProjectWorldToScreen` (`self.PlayerController`) (`KismetMathLibrary.MakeVector` _location_x _location_y (+ _location_z 75.0))) true))
        (:`then_2`
          (`UserWidget.PlayAnimation` _damagenumber (`/Game/Blueprints/UI/WBP_DamageNumber.TextAnimation` _damagenumber) 0.0 1 "Forward" 1.0 false))
        (:`then_3`
          (`UserWidget.AddToViewport` (`local.DamageNumber`) 0))))
    (:`else`)))

(fn `GetHit`
  (params (InDamage :type "Float (single-precision)"))
  (`self.TakeDamage` InDamage)
  (`self.PlayHitReactAnimation`)
  (`NiagaraFunctionLibrary.SpawnSystemAtLocation` (`self.HitParticles`) (`self.K2_GetActorLocation`))
  (`self.CreateDamageNumber` (`local.InDamage`) (`self.K2_GetActorLocation`)))

(fn `PlayAttackAnim`
  (`PaperZDAnimInstance.K2_PlayAnimationOverride` (`PaperZDAnimationComponent.AnimInstance` (`self.AnimationComponent`)) (`self.AttackAnimSequence`) "DefaultSlot" 1.0 0.0))

(fn `PlayHitReactAnimation`
  (`PaperZDAnimInstance.K2_PlayAnimationOverride` (`PaperZDAnimationComponent.AnimInstance` (`self.AnimationComponent`)) (`self.HitReactAnimSequence`) "DefaultSlot" 1.0 0.0))

(fn `TakeDamage`
  (params (InDamage :type "Float (single-precision)"))
  (set `self.CurrentHealth` (`KismetMathLibrary.FClamp` (- (`self.CurrentHealth`) InDamage) 0.0 (`self.MaxHealth`))))

(fn `UserConstructionScript`)